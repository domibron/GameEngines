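; Goal actor that adds a point to the score whenever something begins overlapping its Box component.
; On BeginPlay it finds the Manager actor with GetActorOfClass, caches the reference and prints its name.
; Each overlap increments FScore on that Manager by one, with no check on the overlapping actor, and prints the new total.
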(event OnComponentBeginOverlap(Box)
  (params (OverlappedComponent :type Primitive%20Component%20Object%20Reference) (OtherActor :type Actor%20Object%20Reference) (OtherComp :type Primitive%20Component%20Object%20Reference) (OtherBodyIndex :type Integer) (bFromSweep :type Boolean) (SweepResult :type Hit%20Result%20Structure%20%28by%20ref%29))
  (bind _manager_class (Variables|Default|Getmanager%20class))
  ;[1 1 1] Collision dectection and point incrementing
  (bind _output_get (Variables|/Game/Blueprints/Old/manager.manager_C|Setf_score _manager_class (+ (Variables|/Game/Blueprints/Old/manager.manager_C|Getf_score _manager_class) 1.0)))
  (Development|PrintString (Utilities|String|ToString(Float) _output_get)))

(event EventBeginPlay
  ;[1 1 1] Init for manager variable
  (bind _returnvalue (Actor|GetActorOfClass "/Game/Blueprints/Old/manager.manager_C"))
  (bind _output_get (Variables|Default|Setmanager%20class _returnvalue))
  (Development|PrintString (Utilities|GetDisplayName _output_get)))

(fn ConstructionScript)
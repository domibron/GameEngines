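; An early player Blueprint with physics-driven movement and a hitscan shot that pushes objects.
; Horizontal and Vertical axes add force to the capsule along the actor's right and forward vectors, while mouse look inputs are left empty.
; Shoot runs an object line trace from the camera with debug drawing, then applies an impulse to the hit component against the impact normal.
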(event EventBeginPlay)

(event Collision|EventActorBeginOverlap
  (params (OtherActor :type Actor%20Object%20Reference)))

(event EventTick
  (params (DeltaSeconds :type Float%20%28single-precision%29)))

(event Input|ActionEvents|InputActionShoot
  (params (Key :type Key%20Structure))
  (bind _camera (Variables|Default|GetCamera))
  (bind _returnvalue (Transformation|GetWorldLocation _camera))
  ;[0.521 0.3309 1] Raycast
  (:Pressed
    (bind (_outhit _returnvalue_2) (Collision|LineTraceForObjects _returnvalue (+ _returnvalue (* (Math|Vector|GetForwardVector (Transformation|GetWorldRotation _camera)) (Variables|Default|GetShootDistance))) (Variables|Default|GetObject%20Types) false 0 "ForDuration" true "(R=1.000000,G=0.000000,B=0.000000,A=1.000000)" "(R=0.000000,G=1.000000,B=0.000000,A=1.000000)" 2e+01))
    (if _returnvalue_2
      (Physics|AddImpulse (.hitcomponent _outhit) (* (* (.impactnormal _outhit) (Variables|Default|GetForce)) -1.0) "None" false))))

(event Input|AxisEvents|InputAxisHorizontal
  (params (AxisValue :type Float%20%28single-precision%29))
  ;[1 1 1] Movmenet
  ;;[1 1 1] Left right movement
  (Physics|AddForce (Variables|Default|GetCapsule) (* (Math|Vector|GetRightVector (Transformation|GetActorRotation)) AxisValue) "None" false))

(event Input|AxisEvents|InputAxisVertical
  (params (AxisValue :type Float%20%28single-precision%29))
  ;[1 1 1] Movmenet
  ;;[1 1 1] Forward back movement
  (Physics|AddForce (Variables|Default|GetCapsule) (* (Math|Vector|GetForwardVector (Transformation|GetActorRotation)) AxisValue) "None" false))

(event Input|AxisEvents|InputAxisMouseX
  (params (AxisValue :type Float%20%28single-precision%29))
  ;[1 1 1] look
  ;;[1 0.4 0.7894] Left right look
)

(event Input|AxisEvents|InputAxisMouseY
  (params (AxisValue :type Float%20%28single-precision%29))
  ;[1 1 1] look
  ;;[1 1 1] Up down look
)

(fn ConstructionScript)
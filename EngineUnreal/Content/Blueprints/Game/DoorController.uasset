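; DoorController is an exit door actor that loads another level once the score reaches the total possible.
; On BeginPlay it finds and caches the level's ScoreManager.
; When any actor overlaps it, it compares that manager's Score to TotalScorePossible.
; If the score is equal or greater, it opens the level named by LevelName and prints a debug string.
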(event EventBeginPlay
  (bind _returnvalue (Actor|GetActorOfClass "/Game/Blueprints/Game/ScoreManager.ScoreManager_C"))
  (Variables|Default|SetScoreManagerRef _returnvalue))

(event Collision|EventActorBeginOverlap
  (params (OtherActor :type Actor%20Object%20Reference))
  (bind _scoremanagerref (Variables|Default|GetScoreManagerRef))
  (Math|Integer|CompareInt (Variables|/Game/Blueprints/Game/ScoreManager.ScoreManager_C|GetScore _scoremanagerref) (Variables|/Game/Blueprints/Game/ScoreManager.ScoreManager_C|GetTotalScorePossible _scoremanagerref)
    (:>
      _)
    (:==
      _))
  (Game|OpenLevel(byName) (Utilities|String|StringToName (Variables|Default|GetLevelName)))
  (Development|PrintString "Hello"))

(fn ConstructionScript)
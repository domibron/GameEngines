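; Coin is a collectible actor that adds one point to the score when overlapped.
; On BeginPlay it finds the ScoreManager with GetActorOfClass, caches the reference and increments TotalScorePossible, so each coin registers itself in the maximum score.
; Any actor overlap increments the manager's Score and destroys the coin, with no check on which actor overlapped.
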(event EventBeginPlay
  (bind _returnvalue (Actor|GetActorOfClass "/Game/Blueprints/Game/ScoreManager.ScoreManager_C"))
  (bind _output_get (Variables|Default|SetScoreManagerRef _returnvalue))
  (Variables|/Game/Blueprints/Game/ScoreManager.ScoreManager_C|SetTotalScorePossible _output_get (+ (Variables|/Game/Blueprints/Game/ScoreManager.ScoreManager_C|GetTotalScorePossible _output_get) 1)))

(event Collision|EventActorBeginOverlap
  (params (OtherActor :type Actor%20Object%20Reference))
  (bind _scoremanagerref (Variables|Default|GetScoreManagerRef))
  (Variables|/Game/Blueprints/Game/ScoreManager.ScoreManager_C|SetScore _scoremanagerref (+ (Variables|/Game/Blueprints/Game/ScoreManager.ScoreManager_C|GetScore _scoremanagerref) 1))
  (Actor|DestroyActor))

(fn ConstructionScript)